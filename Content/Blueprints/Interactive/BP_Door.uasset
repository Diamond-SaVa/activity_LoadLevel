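; BP_Door is an interactable door that walks the player through it while streaming levels between its two sides.
; Overlap triggers SideA and SideB record the player's side, which selects the destination and level to load.
; Interact disables collision and input, plays the open animation and lerps the pawn across on a timeline.
; On finish it closes, restores both and unloads the level selected by the re-read side flag.
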(event `self.ReceiveBeginPlay`
  (add `PrimitiveComponent.OnComponentBeginOverlap` (`self.SideA`) (delegate `OnOverlapSideA`))
  (add `PrimitiveComponent.OnComponentBeginOverlap` (`self.SideB`) (delegate `OnOverlapSideB`)))

(event `OnOverlapSideA`
  (params (OverlappedComponent :type "PrimitiveComponent Object Reference") (OtherActor :type "Actor Object Reference") (OtherComp :type "PrimitiveComponent Object Reference") (OtherBodyIndex :type Integer) (bFromSweep :type Boolean) (SweepResult :type "HitResult Structure (by ref)"))
  (set `self.bFromSideA` true))

(event `OnOverlapSideB`
  (params (OverlappedComponent :type "PrimitiveComponent Object Reference") (OtherActor :type "Actor Object Reference") (OtherComp :type "PrimitiveComponent Object Reference") (OtherBodyIndex :type Integer) (bFromSweep :type Boolean) (SweepResult :type "HitResult Structure (by ref)"))
  (set `self.bFromSideA` false))

(event `self.ReceiveEndPlay`
  (params (EndPlayReason :type "EEndPlayReason Enum" :default "Destroyed"))
  (clear `PrimitiveComponent.OnComponentBeginOverlap` (`self.SideA`))
  (clear `PrimitiveComponent.OnComponentBeginOverlap` (`self.SideB`)))

(event `/Game/Blueprints/Interfaces/BPI_Interact.Interact`
  (params (PlayerWhoInteracted :type "Pawn Soft Object Reference"))
  (bind (_movetolocation_x _movetolocation_y) (`KismetMathLibrary.BreakVector` (`self.movetoLocation`)))
  (bind _returnvalue (`self.K2_GetActorLocation` (`self.PlayerPawn`)))
  ; Sets and Validates Player
  (bind _output_get (set `self.PlayerCharacter` PlayerWhoInteracted))
  (if (`KismetSystemLibrary.IsValidSoftObjectReference` _output_get)
    (bind _object (`|LoadAsset` (`self.PlayerCharacter`))
      (:`then`
        (bind _aspawn (cast `Pawn` _object))
        (set `self.PlayerPawn` _aspawn)
        (set `self.movetoLocation` (select `bool` (not (`self.bFromSideA`)) :`false` (`SceneComponent.K2_GetComponentLocation` (`self.SideB`)) :`true` (`SceneComponent.K2_GetComponentLocation` (`self.SideA`))))
        ; Loads Other Level and Makes Player Walk to the Other Side of Door
        (`PrimitiveComponent.SetCollisionEnabled` (`self.BoxCollision`) "NoCollision")
        (`GameplayStatics.LoadStreamLevelBySoftObjectPtr` (select `bool` (not (`self.bFromSideA`)) :`false` (`self.LevelFromB`) :`true` (`self.LevelFromA`)) true)
        (`self.DisableInput` (`self.PlayerPawn`) (`GameplayStatics.GetPlayerController` 0))
        (`SkeletalMeshComponent.PlayAnimation` (`self.SM_Door`) "/Game/SkeletalMeshes/DungeonLayout/anim_modungeon_door_open.anim_modungeon_door_open" false)
        (bind (_direction _lerp) (`Timeline|LerpPlayerTo` :!via `PlayFromStart`)
          (:`Update`
            (`self.K2_SetActorLocation` (`self.PlayerPawn`) (`KismetMathLibrary.VLerp` _returnvalue (`KismetMathLibrary.MakeVector` _movetolocation_x _movetolocation_y (.z _returnvalue)) _lerp) false false))
          (:`Finished`
            ; Opens and Closes Door
            (`self.EnableInput` (`self.PlayerPawn`) (`GameplayStatics.GetPlayerController` 0))
            (`SkeletalMeshComponent.PlayAnimation` (`self.SM_Door`) "/Game/SkeletalMeshes/DungeonLayout/anim_modungeon_door_close.anim_modungeon_door_close" false)
            (`GameplayStatics.UnloadStreamLevelBySoftObjectPtr` (select `bool` (not (`self.bFromSideA`)) :`false` (`self.LevelFromB`) :`true` (`self.LevelFromA`)))
            (`PrimitiveComponent.SetCollisionEnabled` (`self.BoxCollision`) "QueryAndPhysics")
            (set `self.PlayerPawn` null)))))))

(fn `UserConstructionScript`)